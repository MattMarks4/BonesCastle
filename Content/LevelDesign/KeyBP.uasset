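; KeyBP is a key pickup actor that spins and bobs in place until the player character touches it.
; A self-restarting timeline moves the mesh along Z, while Tick yaws the root by a fixed, frame-rate-dependent step.
; Sphere overlap with MyCharacterBP plays a pickup sound and destroys the actor, without recording the key on the character.
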(event OnComponentBeginOverlap(Sphere)
  (params (OverlappedComponent :type Primitive%20Component%20Object%20Reference) (OtherActor :type Actor%20Object%20Reference) (OtherComp :type Primitive%20Component%20Object%20Reference) (OtherBodyIndex :type Integer) (bFromSweep :type Boolean) (SweepResult :type Hit%20Result%20Structure%20%28by%20ref%29))
  (Utilities|Casting|CastToMyCharacterBP OtherActor)
  (Audio|PlaySoundatLocation "/Game/Sounds/pickup_Cue.pickup_Cue" (Transformation|GetActorLocation) "0, 0, 0" 1.0 1.0 0.0 0 0 0)
  (Actor|DestroyActor))

(event Custom|swing
  (bind _swing (Timeline|Timeline_0 PlayFromStart)
    (:Update
      (Transformation|SetRelativeLocation (Variables|Default|GetStaticMesh) (Math|Vector|Lerp(Vector) "0, 0, 0" "0.000000,0.000000,100.000000" _swing) false false))
    (:Finished
      (CallFunction|Swing))))

(event EventBeginPlay
  (CallFunction|Swing))

(event Collision|EventActorBeginOverlap
  (params (OtherActor :type Actor%20Object%20Reference)))

(event EventTick
  (params (DeltaSeconds :type Float%20%28single-precision%29))
  (Transformation|AddLocalRotation (Variables|Default|GetDefaultSceneRoot) (Math|Rotator|MakeRotator 0.0 0.0 3.0) false false))

(fn ConstructionScript)